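; House assembly reveal actor that makes its static mesh parts appear from bottom to top over a set duration.
; BeginPlay caches the parts and actor bounds, then hides every part, or prints an error and stops ticking if the duration is not positive.
; Tick raises a height threshold, shows parts whose bottom lies below it, draws a thin cyan debug box there, and stops ticking when finished.
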(event EventBeginPlay
  (bind _self self)
  (bind _returnvalue (Actor|GetComponentsByClass _self "/Script/Engine.StaticMeshComponent"))
  (bind (_origin _boxextent) (Collision|GetActorBounds _self false false))
  ;[0.15 0.15 0.15 0.5] Comment
  (Variables|运行数据|SetAssemblyElapsed 0.0)
  (Variables|运行数据|SetPartComponents _returnvalue)
  (Variables|运行数据|SetAssemblyCenter _origin)
  (Variables|运行数据|SetAssemblyExtent _boxextent)
  (Variables|运行数据|SetAssemblyBottomZ (- (.Z (Math|Vector|BreakVector _origin)) (.Z (Math|Vector|BreakVector _boxextent))))
  (Variables|运行数据|SetAssemblyTopZ (+ (.Z (Math|Vector|BreakVector _origin)) (.Z (Math|Vector|BreakVector _boxextent))))
  (if (> (Variables|特效参数|GetAssemblyDuration) (Math|Float|MakeLiteralFloat 0.0))
    (for _array_element _returnvalue
      (bind _asscene_component (Utilities|Casting|CastToSceneComponent _array_element)
        (:then
          (Rendering|SetVisibility _asscene_component false false))
        (:CastFailed
          (Development|PrintString "装配特效初始化失败：模型部件无法转换为场景组件。" true true "(R=0.000000,G=0.660000,B=1.000000,A=1.000000)" 5.0))))
    (else
      (Development|PrintString "装配特效参数错误：AssemblyDuration 必须大于 0 秒。" true true "(R=0.000000,G=0.660000,B=1.000000,A=1.000000)" 5.0)
      (Actor|Tick|SetActorTickEnabled _self))))

(event Collision|EventActorBeginOverlap
  (params (OtherActor :type Actor%20Object%20Reference)))

(event EventTick
  (params (DeltaSeconds :type Float%20%28single-precision%29))
  (Variables|运行数据|SetAssemblyElapsed (+ (Variables|运行数据|GetAssemblyElapsed) DeltaSeconds))
  (for _array_element (Variables|运行数据|GetPartComponents)
    (bind _asscene_component (Utilities|Casting|CastToSceneComponent _array_element)
      (:then
        (Rendering|SetVisibility _asscene_component (<= (- (.Z (Math|Vector|BreakVector (.Origin (Collision|GetComponentBounds _asscene_component)))) (.Z (Math|Vector|BreakVector (.BoxExtent (Collision|GetComponentBounds _asscene_component))))) (+ (Variables|运行数据|GetAssemblyBottomZ) (* (- (Variables|运行数据|GetAssemblyTopZ) (Variables|运行数据|GetAssemblyBottomZ)) (Math|Float|Clamp(Float) (/ (Variables|运行数据|GetAssemblyElapsed) (Variables|特效参数|GetAssemblyDuration)))))) false))
      (:CastFailed
        (Development|PrintString "装配特效运行失败：模型部件无法转换为场景组件。" true true "(R=0.000000,G=0.660000,B=1.000000,A=1.000000)" 5.0))))
  (Rendering|Debug|DrawDebugBox (Math|Vector|MakeVector (.X (Math|Vector|BreakVector (Variables|运行数据|GetAssemblyCenter))) (.Y (Math|Vector|BreakVector (Variables|运行数据|GetAssemblyCenter))) (+ (Variables|运行数据|GetAssemblyBottomZ) (* (- (Variables|运行数据|GetAssemblyTopZ) (Variables|运行数据|GetAssemblyBottomZ)) (Math|Float|Clamp(Float) (/ (Variables|运行数据|GetAssemblyElapsed) (Variables|特效参数|GetAssemblyDuration)))))) (Math|Vector|MakeVector (.X (Math|Vector|BreakVector (Variables|运行数据|GetAssemblyExtent))) (.Y (Math|Vector|BreakVector (Variables|运行数据|GetAssemblyExtent))) 2.0) (Utilities|Struct|MakeLinearColor 0.15 0.85 1.0 1.0) "0, 0, 0" 0.05 2.0)
  (if (>= (Math|Float|Clamp(Float) (/ (Variables|运行数据|GetAssemblyElapsed) (Variables|特效参数|GetAssemblyDuration))) (Math|Float|MakeLiteralFloat 1.0))
    (Actor|Tick|SetActorTickEnabled self)))

(fn ConstructionScript)