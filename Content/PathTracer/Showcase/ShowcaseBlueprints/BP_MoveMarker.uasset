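; BP_MoveMarker is a marker actor that flashes an animated wave plane at a given move location in the path tracer showcase.
; BeginPlay puts a dynamic M_PT_Mark_Wave material on the plane and caches the demo player controller.
; EventMoveMarker moves and shows the actor, then a timeline drives material opacity while rescaling the plane by clamped camera distance, hiding it when finished.
; SetMoveMarkerColor tints the material.
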(event Custom|EventMoveMarker
  (params (Location :type Vector))
  (bind _returnvalue (Transformation|GetActorLocation))
  (bind _playercontroller (Variables|Default|GetPlayerController))
  (bind _playercharacter (Variables|/Game/PathTracer/Showcase/ShowcaseBlueprints/PC_DemoPlayerController.PC_DemoPlayerController_C|GetPlayerCharacter _playercontroller))
  (bind _camera (Variables|/Game/PathTracer/Showcase/ShowcaseBlueprints/BP_DemoCharacter.BP_DemoCharacter_C|GetCamera _playercharacter))
  (bind _returnvalue_2 (Transformation|GetWorldLocation _camera))
  (bind _returnvalue_3 (- _returnvalue _returnvalue_2))
  (bind _returnvalue_4 (Math|Vector|VectorLength _returnvalue_3))
  (bind _returnvalue_5 (/ _returnvalue_4 2e+03))
  (bind _returnvalue_6 (Math|Float|Clamp(Float) _returnvalue_5 1.2 3.0))
  (bind _returnvalue_7 (Math|Conversions|ToVector(Float) _returnvalue_6))
  (Transformation|SetActorLocation Location false false)
  (Transformation|SetWorldScale3D (Variables|Default|GetPlane) _returnvalue_7)
  (Rendering|SetActorHiddenInGame false)
  (bind _time (Timeline|MoveAnim PlayFromStart)
    (:Update
      (Rendering|Material|SetScalarParameterValue (Variables|Default|GetCirclesMaterial) "Opacity" _time :!class /Script/Engine.MaterialInstanceDynamic)
      (Transformation|SetWorldScale3D (Variables|Default|GetPlane) _returnvalue_7))
    (:Finished
      (Rendering|SetActorHiddenInGame true)
      (Transformation|SetWorldScale3D (Variables|Default|GetPlane) "1.000000,1.000000,1.000000"))))

(event EventBeginPlay
  (bind _returnvalue (Rendering|Material|CreateDynamicMaterialInstance "/Game/PathTracer/Materials/Path_Marks/M_PT_Mark_Wave.M_PT_Mark_Wave" "None" "None" :!class /Script/Engine.KismetMaterialLibrary))
  (Variables|Default|SetCirclesMaterial _returnvalue)
  (Rendering|Material|SetMaterial (Variables|Default|GetPlane) 0 _returnvalue)
  (bind _returnvalue_2 (Actor|GetActorOfClass "/Game/PathTracer/Showcase/ShowcaseBlueprints/PC_DemoPlayerController.PC_DemoPlayerController_C"))
  (Variables|Default|SetPlayerController _returnvalue_2))

(fn ConstructionScript)

(fn SetMoveMarkerColor
  (params (Color :type Linear%20Color%20Structure))
  (Rendering|Material|SetVectorParameterValue (Variables|Default|GetCirclesMaterial) "Color" Color :!class /Script/Engine.MaterialInstanceDynamic))