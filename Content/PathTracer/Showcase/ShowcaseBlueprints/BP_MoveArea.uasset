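; BP_MoveArea outlines the cells reachable within a move distance on a BP_Grid, drawing the area's border with path tracers.
; UpdateBorder runs a breadth-first flood fill over passable neighbors, recording directed edges where expansion is blocked or move points run out.
; Those edges are chained into closed loops, using direction to resolve shared corners.
; Each loop is drawn by a pooled BP_PathTracer child actor, hidden and reused between updates.
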(fn ConstructionScript)

(fn UpdateBorder
  (params (StartLocation :type Vector) (MoveDistance :type Integer))
  (Utilities|IsValid (Variables|Default|GetGridActor)
    (:Is%20Valid
      _)
    (:Is%20Not%20Valid
      (bind _returnvalue (Actor|GetActorOfClass "/Game/PathTracer/Showcase/ShowcaseBlueprints/BP_Grid.BP_Grid_C"))
      (Variables|Default|SetGridActor _returnvalue)))
  (Private|ResetPathTrecers)
  (Private|SetStartMoveGridCell StartLocation MoveDistance)
  (Private|FindBorderPoints)
  (Private|FilteredPointsandDrawBorder))

(fn DrawBorder
  (params (GridPoints :type Array%20of%20Integers))
  (if (> (Utilities|Array|Length GridPoints) 1)
    (for _array_element GridPoints
      (Utilities|Array|Add (LocalVariables|GetGridPointsLocationsLOCAL) (Default|GetGridNodesWorldCoordinates (Variables|Default|GetGridActor) _array_element)))
    (bind _pathtracer (Private|GetPathTracer))
    (Default|DrawPath _pathtracer (LocalVariables|GetGridPointsLocationsLOCAL))))

(fn SetStartMoveGridCell
  (params (Location :type Vector) (Move%20DIstance :type Integer))
  (Variables|Default|SetStartCellNumber (Math|Integer|Clamp(Integer) (Default|GetCellNumberbyWorldLocation (Variables|Default|GetGridActor) (Math|Conversions|ToVector2D(Vector) Location)) 1 (Variables|/Game/PathTracer/Showcase/ShowcaseBlueprints/BP_Grid.BP_Grid_C|GetCellsCount (Variables|Default|GetGridActor))))
  (Variables|Default|SetMoveDistance (Math|Integer|Clamp(Integer) Move%20DIstance 0 Move%20DIstance)))

(fn FindBorderPoints
  (bind _cellsforvisitlocal (LocalVariables|GetCellsForVisitLOCAL))
  (bind _output (Utilities|Array|Get(acopy) _cellsforvisitlocal))
  (bind (_x _y) (Utilities|Struct|BreakIntPoint _output))
  ;[0.09538 0.5938 0 0.15 16] Setup before reuse
  (Utilities|Array|Clear (Variables|Default|GetConnectedWith))
  (Utilities|Array|Clear (Variables|Default|GetCrossPoints))
  (Utilities|Array|Clear (Variables|Default|GetCellsInArea))
  (Utilities|Array|Clear (Variables|Default|GetDuplicatePoints))
  (if (.Passable (Utilities|Struct|BreakS_GridCellData (Utilities|Array|Get(acopy) (Variables|/Game/PathTracer/Showcase/ShowcaseBlueprints/BP_Grid.BP_Grid_C|GetGridData (Variables|Default|GetGridActor)) (- (Variables|Default|GetStartCellNumber) 1)))) ; Is the starting cell passable?
    (Utilities|Array|Add (LocalVariables|GetCellsForVisitLOCAL) (Utilities|Struct|MakeIntPoint (Variables|Default|GetStartCellNumber) (Variables|Default|GetMoveDistance))) ; Set start Cell
    (Utilities|Array|SetArrayElem (LocalVariables|GetVisitedCellsLOCAL) (Utilities|Array|LastIndex (Variables|/Game/PathTracer/Showcase/ShowcaseBlueprints/BP_Grid.BP_Grid_C|GetGridData (Variables|Default|GetGridActor))) false true) ; Make empty array
    (Utilities|Array|SetArrayElem (LocalVariables|GetVisitedCellsLOCAL) (- (Variables|Default|GetStartCellNumber) 1) true) ; Set Start Cell is visited
    ;[0.09538 0.5938 0 0.15 16] Need to visit all available cells
    ; If there are no cells left, then its are all visited
    (while (> (Utilities|Array|Length (LocalVariables|GetCellsForVisitLOCAL)) 0)
      (LocalVariables|SetCurrentCellLOCAL _x)
      (LocalVariables|SetRemainderOfMovePointsLOCAL _y)
      (bind _neighboringcells (Default|GetNeighboringCells (Variables|Default|GetGridActor) (LocalVariables|GetCurrentCellLOCAL)))
      (for _index (range 0 3) ; Check Left, Top, Right and Bottom neighbor Cells
        (LocalVariables|SetDirectionLOCAL _index)
        (LocalVariables|SetNeighborCellNumberLOCAL (Utilities|Select :Index _index :Option%200 (.Left (Utilities|Struct|BreakIntMargin _neighboringcells)) :Option%201 (.Top (Utilities|Struct|BreakIntMargin _neighboringcells)) :Option%202 (.Right (Utilities|Struct|BreakIntMargin _neighboringcells)) :Option%203 (.Bottom (Utilities|Struct|BreakIntMargin _neighboringcells))))
        ;[0.09538 0.5938 0 0.15 16] Checking the next Cell to bypass
        (if (!= (LocalVariables|GetNeighborCellNumberLOCAL) -1) ; Check if a Cell is within the Grid
          (if (not (Utilities|Array|Get(acopy) (LocalVariables|GetVisitedCellsLOCAL) (- (LocalVariables|GetNeighborCellNumberLOCAL) 1))) ; If cell not visited
            (if (> (LocalVariables|GetRemainderOfMovePointsLOCAL) 0) ; Has Move Points
              (if (.Passable (Utilities|Struct|BreakS_GridCellData (Utilities|Array|Get(acopy) (Variables|/Game/PathTracer/Showcase/ShowcaseBlueprints/BP_Grid.BP_Grid_C|GetGridData (Variables|Default|GetGridActor)) (- (LocalVariables|GetNeighborCellNumberLOCAL) 1)))) ; Is Target Cell Passable
                ;[0.09538 0.5938 0 0.15 16] If successful, add a new cell to the array for future visits
                ; And mark as visited so that other cells cannot add copy of it
                (Utilities|Array|Add (LocalVariables|GetCellsForVisitLOCAL) (Utilities|Struct|MakeIntPoint (LocalVariables|GetNeighborCellNumberLOCAL) (- (LocalVariables|GetRemainderOfMovePointsLOCAL) 1)))
                (Utilities|Array|SetArrayElem (LocalVariables|GetVisitedCellsLOCAL) (- (LocalVariables|GetNeighborCellNumberLOCAL) 1) true)
                (Utilities|Array|Add (Variables|Default|GetCellsInArea) (LocalVariables|GetNeighborCellNumberLOCAL))
                (else
                  (Private|AddCellEdgetoDrawBorder (LocalVariables|GetCurrentCellLOCAL) (LocalVariables|GetDirectionLOCAL))))
              (else
                (Private|AddCellEdgetoDrawBorder (LocalVariables|GetCurrentCellLOCAL) (LocalVariables|GetDirectionLOCAL)))))
          (else
            (Private|AddCellEdgetoDrawBorder (LocalVariables|GetCurrentCellLOCAL) (LocalVariables|GetDirectionLOCAL)))))
      (Utilities|Array|RemoveIndex (LocalVariables|GetCellsForVisitLOCAL)))))

(fn FilteredPointsandDrawBorder
  ;[0.09538 0.5938 0 0.15 16] As long as there are points to bypass the perimeter, the loop is executed
  (while (> (Utilities|Array|Length (Variables|Default|GetCrossPoints)) 0)
    ;[0.09538 0.5938 0 0.15 16] Setup before reuse
    (Utilities|Array|Clear (LocalVariables|GetBorderLOCAL))
    (LocalVariables|SetNextPointLOCAL (Utilities|Array|Get(acopy) (Variables|Default|GetCrossPoints)))
    (LocalVariables|SetLastDirectionLOCAL -1)
    (LocalVariables|SetLastIndexLOCAL (Utilities|Array|LastIndex (Variables|Default|GetCrossPoints)))
    (Utilities|FlowControl|ForLoopwithBreak 0 (LocalVariables|GetLastIndexLOCAL) :!label _label
      (:LoopBody
        (LocalVariables|SetCurrentPointLOCAL (LocalVariables|GetNextPointLOCAL))
        (if (>= (Utilities|Array|FindItem (Variables|Default|GetCrossPoints) (LocalVariables|GetCurrentPointLOCAL)) 0) ; If the value is not found, then the border is looped
          (LocalVariables|SetCurrentPointIndexLOCAL (Utilities|Array|FindItem (Variables|Default|GetCrossPoints) (LocalVariables|GetCurrentPointLOCAL)))
          (Utilities|FlowControl|Sequence
            (:then_0
              (LocalVariables|SetDuplicatePointIndexLOCAL (Utilities|Array|FindItem (Variables|Default|GetDuplicatePoints) (LocalVariables|GetCurrentPointLOCAL)))
              (if (>= (LocalVariables|GetDuplicatePointIndexLOCAL) 0)
                (Utilities|Array|RemoveIndex (Variables|Default|GetDuplicatePoints) (LocalVariables|GetDuplicatePointIndexLOCAL))
                (if (== (LocalVariables|GetLastDirectionLOCAL) (Math|Integer|SelectInt 0 (+ (Utilities|Struct|BreakS_RibData (Utilities|Array|Get(acopy) (Variables|Default|GetConnectedWith) (LocalVariables|GetCurrentPointIndexLOCAL))) 1) (== (+ (Utilities|Struct|BreakS_RibData (Utilities|Array|Get(acopy) (Variables|Default|GetConnectedWith) (LocalVariables|GetCurrentPointIndexLOCAL))) 1) 4)))
                  ;[0.09538 0.5938 0 0.15 14] Find second duplicate point in array
                  (Utilities|Array|SetArrayElem (Variables|Default|GetCrossPoints) (LocalVariables|GetCurrentPointIndexLOCAL) (+ (LocalVariables|GetCurrentPointLOCAL) 1))
                  (LocalVariables|SetDuplicatePointIndexLOCAL (Utilities|Array|FindItem (Variables|Default|GetCrossPoints) (LocalVariables|GetCurrentPointLOCAL))) ; Reuse variable
                  (Utilities|Array|SetArrayElem (Variables|Default|GetCrossPoints) (LocalVariables|GetCurrentPointIndexLOCAL) (LocalVariables|GetCurrentPointLOCAL))
                  (LocalVariables|SetCurrentPointIndexLOCAL (LocalVariables|GetDuplicatePointIndexLOCAL)))))
            (:then_1
              ;[0.09538 0.5938 0 0.15 14] If the past Rib has the same direction as the new Rib,
              ; the point can be skipped to reduce the number of Border segments and improve performance.
              (LocalVariables|SetNextPointLOCAL (.ConnectedPointsNumbers (Utilities|Struct|BreakS_RibData (Utilities|Array|Get(acopy) (Variables|Default|GetConnectedWith) (LocalVariables|GetCurrentPointIndexLOCAL)))))
              (if (== (LocalVariables|GetLastDirectionLOCAL) (.Direction (Utilities|Struct|BreakS_RibData (Utilities|Array|Get(acopy) (Variables|Default|GetConnectedWith) (LocalVariables|GetCurrentPointIndexLOCAL)))))
                _
                (else
                  _))
              (LocalVariables|SetLastDirectionLOCAL (.Direction (Utilities|Struct|BreakS_RibData (Utilities|Array|Get(acopy) (Variables|Default|GetConnectedWith) (LocalVariables|GetCurrentPointIndexLOCAL)))))
              (Utilities|Array|Add (LocalVariables|GetBorderLOCAL) (LocalVariables|GetCurrentPointLOCAL)))
            (:then_2
              (Utilities|Array|RemoveIndex (Variables|Default|GetCrossPoints) (LocalVariables|GetCurrentPointIndexLOCAL))
              (Utilities|Array|RemoveIndex (Variables|Default|GetConnectedWith) (LocalVariables|GetCurrentPointIndexLOCAL))))
          (else
            (goto _label Break))))
      (:Completed
        (Private|DrawBorder (LocalVariables|GetBorderLOCAL))))))

(fn AddCellEdgetoDrawBorder
  (params (CellNumber :type Integer) (Direction :type Integer))
  (bind _gridactor (Variables|Default|GetGridActor))
  (LocalVariables|SetCellNumLOCAL CellNumber)
  (LocalVariables|SetDirectionLOCAL Direction)
  ;[0.09538 0.5938 0 0.15 16] Each point can have a maximum of 2 connected neighboring points
  ; All duplicates are added to the array
  (LocalVariables|SetPointAlreadyInArrayLOCAL (>= (Utilities|Array|FindItem (Variables|Default|GetCrossPoints) (.X (Utilities|Struct|BreakIntPoint (Utilities|Select :Index (LocalVariables|GetDirectionLOCAL) :Option%200 (Utilities|Struct|MakeIntPoint (Utilities|Select :Index (LocalVariables|GetDirectionLOCAL) :Option%200 (+ (.X (Utilities|Struct|BreakIntPoint (Default|GetGridCoordinatesbyCellNum _gridactor (LocalVariables|GetCellNumLOCAL)))) (.Y (Utilities|Struct|BreakIntPoint (Variables|/Game/PathTracer/Showcase/ShowcaseBlueprints/BP_Grid.BP_Grid_C|GetGridSize _gridactor))) (LocalVariables|GetCellNumLOCAL)) :Option%201 (+ (+ (LocalVariables|GetCellNumLOCAL) (- (.X (Utilities|Struct|BreakIntPoint (Default|GetGridCoordinatesbyCellNum _gridactor (LocalVariables|GetCellNumLOCAL)))) 1)) 1) :Option%202 (+ (+ (.X (Utilities|Struct|BreakIntPoint (Default|GetGridCoordinatesbyCellNum _gridactor (LocalVariables|GetCellNumLOCAL)))) (.Y (Utilities|Struct|BreakIntPoint (Variables|/Game/PathTracer/Showcase/ShowcaseBlueprints/BP_Grid.BP_Grid_C|GetGridSize _gridactor))) (LocalVariables|GetCellNumLOCAL)) 1) :Option%203 (+ (+ (.X (Utilities|Struct|BreakIntPoint (Default|GetGridCoordinatesbyCellNum _gridactor (LocalVariables|GetCellNumLOCAL)))) (.Y (Utilities|Struct|BreakIntPoint (Variables|/Game/PathTracer/Showcase/ShowcaseBlueprints/BP_Grid.BP_Grid_C|GetGridSize _gridactor))) (LocalVariables|GetCellNumLOCAL)) 1)) (Utilities|Select :Index (LocalVariables|GetDirectionLOCAL) :Option%200 (+ (LocalVariables|GetCellNumLOCAL) (- (.X (Utilities|Struct|BreakIntPoint (Default|GetGridCoordinatesbyCellNum _gridactor (LocalVariables|GetCellNumLOCAL)))) 1)) :Option%201 (+ (LocalVariables|GetCellNumLOCAL) (- (.X (Utilities|Struct|BreakIntPoint (Default|GetGridCoordinatesbyCellNum _gridactor (LocalVariables|GetCellNumLOCAL)))) 1)) :Option%202 (+ (+ (LocalVariables|GetCellNumLOCAL) (- (.X (Utilities|Struct|BreakIntPoint (Default|GetGridCoordinatesbyCellNum _gridactor (LocalVariables|GetCellNumLOCAL)))) 1)) 1) :Option%203 (+ (.X (Utilities|Struct|BreakIntPoint (Default|GetGridCoordinatesbyCellNum _gridactor (LocalVariables|GetCellNumLOCAL)))) (.Y (Utilities|Struct|BreakIntPoint (Variables|/Game/PathTracer/Showcase/ShowcaseBlueprints/BP_Grid.BP_Grid_C|GetGridSize _gridactor))) (LocalVariables|GetCellNumLOCAL)))) :Option%201 (Utilities|Struct|MakeIntPoint (Utilities|Select :Index (LocalVariables|GetDirectionLOCAL) :Option%200 (+ (LocalVariables|GetCellNumLOCAL) (- (.X (Utilities|Struct|BreakIntPoint (Default|GetGridCoordinatesbyCellNum _gridactor (LocalVariables|GetCellNumLOCAL)))) 1)) :Option%201 (+ (LocalVariables|GetCellNumLOCAL) (- (.X (Utilities|Struct|BreakIntPoint (Default|GetGridCoordinatesbyCellNum _gridactor (LocalVariables|GetCellNumLOCAL)))) 1)) :Option%202 (+ (+ (LocalVariables|GetCellNumLOCAL) (- (.X (Utilities|Struct|BreakIntPoint (Default|GetGridCoordinatesbyCellNum _gridactor (LocalVariables|GetCellNumLOCAL)))) 1)) 1) :Option%203 (+ (.X (Utilities|Struct|BreakIntPoint (Default|GetGridCoordinatesbyCellNum _gridactor (LocalVariables|GetCellNumLOCAL)))) (.Y (Utilities|Struct|BreakIntPoint (Variables|/Game/PathTracer/Showcase/ShowcaseBlueprints/BP_Grid.BP_Grid_C|GetGridSize _gridactor))) (LocalVariables|GetCellNumLOCAL))) (Utilities|Select :Index (LocalVariables|GetDirectionLOCAL) :Option%200 (+ (.X (Utilities|Struct|BreakIntPoint (Default|GetGridCoordinatesbyCellNum _gridactor (LocalVariables|GetCellNumLOCAL)))) (.Y (Utilities|Struct|BreakIntPoint (Variables|/Game/PathTracer/Showcase/ShowcaseBlueprints/BP_Grid.BP_Grid_C|GetGridSize _gridactor))) (LocalVariables|GetCellNumLOCAL)) :Option%201 (+ (+ (LocalVariables|GetCellNumLOCAL) (- (.X (Utilities|Struct|BreakIntPoint (Default|GetGridCoordinatesbyCellNum _gridactor (LocalVariables|GetCellNumLOCAL)))) 1)) 1) :Option%202 (+ (+ (.X (Utilities|Struct|BreakIntPoint (Default|GetGridCoordinatesbyCellNum _gridactor (LocalVariables|GetCellNumLOCAL)))) (.Y (Utilities|Struct|BreakIntPoint (Variables|/Game/PathTracer/Showcase/ShowcaseBlueprints/BP_Grid.BP_Grid_C|GetGridSize _gridactor))) (LocalVariables|GetCellNumLOCAL)) 1) :Option%203 (+ (+ (.X (Utilities|Struct|BreakIntPoint (Default|GetGridCoordinatesbyCellNum _gridactor (LocalVariables|GetCellNumLOCAL)))) (.Y (Utilities|Struct|BreakIntPoint (Variables|/Game/PathTracer/Showcase/ShowcaseBlueprints/BP_Grid.BP_Grid_C|GetGridSize _gridactor))) (LocalVariables|GetCellNumLOCAL)) 1))) :Option%202 (Utilities|Struct|MakeIntPoint (Utilities|Select :Index (LocalVariables|GetDirectionLOCAL) :Option%200 (+ (LocalVariables|GetCellNumLOCAL) (- (.X (Utilities|Struct|BreakIntPoint (Default|GetGridCoordinatesbyCellNum _gridactor (LocalVariables|GetCellNumLOCAL)))) 1)) :Option%201 (+ (LocalVariables|GetCellNumLOCAL) (- (.X (Utilities|Struct|BreakIntPoint (Default|GetGridCoordinatesbyCellNum _gridactor (LocalVariables|GetCellNumLOCAL)))) 1)) :Option%202 (+ (+ (LocalVariables|GetCellNumLOCAL) (- (.X (Utilities|Struct|BreakIntPoint (Default|GetGridCoordinatesbyCellNum _gridactor (LocalVariables|GetCellNumLOCAL)))) 1)) 1) :Option%203 (+ (.X (Utilities|Struct|BreakIntPoint (Default|GetGridCoordinatesbyCellNum _gridactor (LocalVariables|GetCellNumLOCAL)))) (.Y (Utilities|Struct|BreakIntPoint (Variables|/Game/PathTracer/Showcase/ShowcaseBlueprints/BP_Grid.BP_Grid_C|GetGridSize _gridactor))) (LocalVariables|GetCellNumLOCAL))) (Utilities|Select :Index (LocalVariables|GetDirectionLOCAL) :Option%200 (+ (.X (Utilities|Struct|BreakIntPoint (Default|GetGridCoordinatesbyCellNum _gridactor (LocalVariables|GetCellNumLOCAL)))) (.Y (Utilities|Struct|BreakIntPoint (Variables|/Game/PathTracer/Showcase/ShowcaseBlueprints/BP_Grid.BP_Grid_C|GetGridSize _gridactor))) (LocalVariables|GetCellNumLOCAL)) :Option%201 (+ (+ (LocalVariables|GetCellNumLOCAL) (- (.X (Utilities|Struct|BreakIntPoint (Default|GetGridCoordinatesbyCellNum _gridactor (LocalVariables|GetCellNumLOCAL)))) 1)) 1) :Option%202 (+ (+ (.X (Utilities|Struct|BreakIntPoint (Default|GetGridCoordinatesbyCellNum _gridactor (LocalVariables|GetCellNumLOCAL)))) (.Y (Utilities|Struct|BreakIntPoint (Variables|/Game/PathTracer/Showcase/ShowcaseBlueprints/BP_Grid.BP_Grid_C|GetGridSize _gridactor))) (LocalVariables|GetCellNumLOCAL)) 1) :Option%203 (+ (+ (.X (Utilities|Struct|BreakIntPoint (Default|GetGridCoordinatesbyCellNum _gridactor (LocalVariables|GetCellNumLOCAL)))) (.Y (Utilities|Struct|BreakIntPoint (Variables|/Game/PathTracer/Showcase/ShowcaseBlueprints/BP_Grid.BP_Grid_C|GetGridSize _gridactor))) (LocalVariables|GetCellNumLOCAL)) 1))) :Option%203 (Utilities|Struct|MakeIntPoint (Utilities|Select :Index (LocalVariables|GetDirectionLOCAL) :Option%200 (+ (.X (Utilities|Struct|BreakIntPoint (Default|GetGridCoordinatesbyCellNum _gridactor (LocalVariables|GetCellNumLOCAL)))) (.Y (Utilities|Struct|BreakIntPoint (Variables|/Game/PathTracer/Showcase/ShowcaseBlueprints/BP_Grid.BP_Grid_C|GetGridSize _gridactor))) (LocalVariables|GetCellNumLOCAL)) :Option%201 (+ (+ (LocalVariables|GetCellNumLOCAL) (- (.X (Utilities|Struct|BreakIntPoint (Default|GetGridCoordinatesbyCellNum _gridactor (LocalVariables|GetCellNumLOCAL)))) 1)) 1) :Option%202 (+ (+ (.X (Utilities|Struct|BreakIntPoint (Default|GetGridCoordinatesbyCellNum _gridactor (LocalVariables|GetCellNumLOCAL)))) (.Y (Utilities|Struct|BreakIntPoint (Variables|/Game/PathTracer/Showcase/ShowcaseBlueprints/BP_Grid.BP_Grid_C|GetGridSize _gridactor))) (LocalVariables|GetCellNumLOCAL)) 1) :Option%203 (+ (+ (.X (Utilities|Struct|BreakIntPoint (Default|GetGridCoordinatesbyCellNum _gridactor (LocalVariables|GetCellNumLOCAL)))) (.Y (Utilities|Struct|BreakIntPoint (Variables|/Game/PathTracer/Showcase/ShowcaseBlueprints/BP_Grid.BP_Grid_C|GetGridSize _gridactor))) (LocalVariables|GetCellNumLOCAL)) 1)) (Utilities|Select :Index (LocalVariables|GetDirectionLOCAL) :Option%200 (+ (LocalVariables|GetCellNumLOCAL) (- (.X (Utilities|Struct|BreakIntPoint (Default|GetGridCoordinatesbyCellNum _gridactor (LocalVariables|GetCellNumLOCAL)))) 1)) :Option%201 (+ (LocalVariables|GetCellNumLOCAL) (- (.X (Utilities|Struct|BreakIntPoint (Default|GetGridCoordinatesbyCellNum _gridactor (LocalVariables|GetCellNumLOCAL)))) 1)) :Option%202 (+ (+ (LocalVariables|GetCellNumLOCAL) (- (.X (Utilities|Struct|BreakIntPoint (Default|GetGridCoordinatesbyCellNum _gridactor (LocalVariables|GetCellNumLOCAL)))) 1)) 1) :Option%203 (+ (.X (Utilities|Struct|BreakIntPoint (Default|GetGridCoordinatesbyCellNum _gridactor (LocalVariables|GetCellNumLOCAL)))) (.Y (Utilities|Struct|BreakIntPoint (Variables|/Game/PathTracer/Showcase/ShowcaseBlueprints/BP_Grid.BP_Grid_C|GetGridSize _gridactor))) (LocalVariables|GetCellNumLOCAL)))))))) 0))
  (Utilities|Array|Add (Variables|Default|GetCrossPoints) (.X (Utilities|Struct|BreakIntPoint (Utilities|Select :Index (LocalVariables|GetDirectionLOCAL) :Option%200 (Utilities|Struct|MakeIntPoint (Utilities|Select :Index (LocalVariables|GetDirectionLOCAL) :Option%200 (+ (.X (Utilities|Struct|BreakIntPoint (Default|GetGridCoordinatesbyCellNum _gridactor (LocalVariables|GetCellNumLOCAL)))) (.Y (Utilities|Struct|BreakIntPoint (Variables|/Game/PathTracer/Showcase/ShowcaseBlueprints/BP_Grid.BP_Grid_C|GetGridSize _gridactor))) (LocalVariables|GetCellNumLOCAL)) :Option%201 (+ (+ (LocalVariables|GetCellNumLOCAL) (- (.X (Utilities|Struct|BreakIntPoint (Default|GetGridCoordinatesbyCellNum _gridactor (LocalVariables|GetCellNumLOCAL)))) 1)) 1) :Option%202 (+ (+ (.X (Utilities|Struct|BreakIntPoint (Default|GetGridCoordinatesbyCellNum _gridactor (LocalVariables|GetCellNumLOCAL)))) (.Y (Utilities|Struct|BreakIntPoint (Variables|/Game/PathTracer/Showcase/ShowcaseBlueprints/BP_Grid.BP_Grid_C|GetGridSize _gridactor))) (LocalVariables|GetCellNumLOCAL)) 1) :Option%203 (+ (+ (.X (Utilities|Struct|BreakIntPoint (Default|GetGridCoordinatesbyCellNum _gridactor (LocalVariables|GetCellNumLOCAL)))) (.Y (Utilities|Struct|BreakIntPoint (Variables|/Game/PathTracer/Showcase/ShowcaseBlueprints/BP_Grid.BP_Grid_C|GetGridSize _gridactor))) (LocalVariables|GetCellNumLOCAL)) 1)) (Utilities|Select :Index (LocalVariables|GetDirectionLOCAL) :Option%200 (+ (LocalVariables|GetCellNumLOCAL) (- (.X (Utilities|Struct|BreakIntPoint (Default|GetGridCoordinatesbyCellNum _gridactor (LocalVariables|GetCellNumLOCAL)))) 1)) :Option%201 (+ (LocalVariables|GetCellNumLOCAL) (- (.X (Utilities|Struct|BreakIntPoint (Default|GetGridCoordinatesbyCellNum _gridactor (LocalVariables|GetCellNumLOCAL)))) 1)) :Option%202 (+ (+ (LocalVariables|GetCellNumLOCAL) (- (.X (Utilities|Struct|BreakIntPoint (Default|GetGridCoordinatesbyCellNum _gridactor (LocalVariables|GetCellNumLOCAL)))) 1)) 1) :Option%203 (+ (.X (Utilities|Struct|BreakIntPoint (Default|GetGridCoordinatesbyCellNum _gridactor (LocalVariables|GetCellNumLOCAL)))) (.Y (Utilities|Struct|BreakIntPoint (Variables|/Game/PathTracer/Showcase/ShowcaseBlueprints/BP_Grid.BP_Grid_C|GetGridSize _gridactor))) (LocalVariables|GetCellNumLOCAL)))) :Option%201 (Utilities|Struct|MakeIntPoint (Utilities|Select :Index (LocalVariables|GetDirectionLOCAL) :Option%200 (+ (LocalVariables|GetCellNumLOCAL) (- (.X (Utilities|Struct|BreakIntPoint (Default|GetGridCoordinatesbyCellNum _gridactor (LocalVariables|GetCellNumLOCAL)))) 1)) :Option%201 (+ (LocalVariables|GetCellNumLOCAL) (- (.X (Utilities|Struct|BreakIntPoint (Default|GetGridCoordinatesbyCellNum _gridactor (LocalVariables|GetCellNumLOCAL)))) 1)) :Option%202 (+ (+ (LocalVariables|GetCellNumLOCAL) (- (.X (Utilities|Struct|BreakIntPoint (Default|GetGridCoordinatesbyCellNum _gridactor (LocalVariables|GetCellNumLOCAL)))) 1)) 1) :Option%203 (+ (.X (Utilities|Struct|BreakIntPoint (Default|GetGridCoordinatesbyCellNum _gridactor (LocalVariables|GetCellNumLOCAL)))) (.Y (Utilities|Struct|BreakIntPoint (Variables|/Game/PathTracer/Showcase/ShowcaseBlueprints/BP_Grid.BP_Grid_C|GetGridSize _gridactor))) (LocalVariables|GetCellNumLOCAL))) (Utilities|Select :Index (LocalVariables|GetDirectionLOCAL) :Option%200 (+ (.X (Utilities|Struct|BreakIntPoint (Default|GetGridCoordinatesbyCellNum _gridactor (LocalVariables|GetCellNumLOCAL)))) (.Y (Utilities|Struct|BreakIntPoint (Variables|/Game/PathTracer/Showcase/ShowcaseBlueprints/BP_Grid.BP_Grid_C|GetGridSize _gridactor))) (LocalVariables|GetCellNumLOCAL)) :Option%201 (+ (+ (LocalVariables|GetCellNumLOCAL) (- (.X (Utilities|Struct|BreakIntPoint (Default|GetGridCoordinatesbyCellNum _gridactor (LocalVariables|GetCellNumLOCAL)))) 1)) 1) :Option%202 (+ (+ (.X (Utilities|Struct|BreakIntPoint (Default|GetGridCoordinatesbyCellNum _gridactor (LocalVariables|GetCellNumLOCAL)))) (.Y (Utilities|Struct|BreakIntPoint (Variables|/Game/PathTracer/Showcase/ShowcaseBlueprints/BP_Grid.BP_Grid_C|GetGridSize _gridactor))) (LocalVariables|GetCellNumLOCAL)) 1) :Option%203 (+ (+ (.X (Utilities|Struct|BreakIntPoint (Default|GetGridCoordinatesbyCellNum _gridactor (LocalVariables|GetCellNumLOCAL)))) (.Y (Utilities|Struct|BreakIntPoint (Variables|/Game/PathTracer/Showcase/ShowcaseBlueprints/BP_Grid.BP_Grid_C|GetGridSize _gridactor))) (LocalVariables|GetCellNumLOCAL)) 1))) :Option%202 (Utilities|Struct|MakeIntPoint (Utilities|Select :Index (LocalVariables|GetDirectionLOCAL) :Option%200 (+ (LocalVariables|GetCellNumLOCAL) (- (.X (Utilities|Struct|BreakIntPoint (Default|GetGridCoordinatesbyCellNum _gridactor (LocalVariables|GetCellNumLOCAL)))) 1)) :Option%201 (+ (LocalVariables|GetCellNumLOCAL) (- (.X (Utilities|Struct|BreakIntPoint (Default|GetGridCoordinatesbyCellNum _gridactor (LocalVariables|GetCellNumLOCAL)))) 1)) :Option%202 (+ (+ (LocalVariables|GetCellNumLOCAL) (- (.X (Utilities|Struct|BreakIntPoint (Default|GetGridCoordinatesbyCellNum _gridactor (LocalVariables|GetCellNumLOCAL)))) 1)) 1) :Option%203 (+ (.X (Utilities|Struct|BreakIntPoint (Default|GetGridCoordinatesbyCellNum _gridactor (LocalVariables|GetCellNumLOCAL)))) (.Y (Utilities|Struct|BreakIntPoint (Variables|/Game/PathTracer/Showcase/ShowcaseBlueprints/BP_Grid.BP_Grid_C|GetGridSize _gridactor))) (LocalVariables|GetCellNumLOCAL))) (Utilities|Select :Index (LocalVariables|GetDirectionLOCAL) :Option%200 (+ (.X (Utilities|Struct|BreakIntPoint (Default|GetGridCoordinatesbyCellNum _gridactor (LocalVariables|GetCellNumLOCAL)))) (.Y (Utilities|Struct|BreakIntPoint (Variables|/Game/PathTracer/Showcase/ShowcaseBlueprints/BP_Grid.BP_Grid_C|GetGridSize _gridactor))) (LocalVariables|GetCellNumLOCAL)) :Option%201 (+ (+ (LocalVariables|GetCellNumLOCAL) (- (.X (Utilities|Struct|BreakIntPoint (Default|GetGridCoordinatesbyCellNum _gridactor (LocalVariables|GetCellNumLOCAL)))) 1)) 1) :Option%202 (+ (+ (.X (Utilities|Struct|BreakIntPoint (Default|GetGridCoordinatesbyCellNum _gridactor (LocalVariables|GetCellNumLOCAL)))) (.Y (Utilities|Struct|BreakIntPoint (Variables|/Game/PathTracer/Showcase/ShowcaseBlueprints/BP_Grid.BP_Grid_C|GetGridSize _gridactor))) (LocalVariables|GetCellNumLOCAL)) 1) :Option%203 (+ (+ (.X (Utilities|Struct|BreakIntPoint (Default|GetGridCoordinatesbyCellNum _gridactor (LocalVariables|GetCellNumLOCAL)))) (.Y (Utilities|Struct|BreakIntPoint (Variables|/Game/PathTracer/Showcase/ShowcaseBlueprints/BP_Grid.BP_Grid_C|GetGridSize _gridactor))) (LocalVariables|GetCellNumLOCAL)) 1))) :Option%203 (Utilities|Struct|MakeIntPoint (Utilities|Select :Index (LocalVariables|GetDirectionLOCAL) :Option%200 (+ (.X (Utilities|Struct|BreakIntPoint (Default|GetGridCoordinatesbyCellNum _gridactor (LocalVariables|GetCellNumLOCAL)))) (.Y (Utilities|Struct|BreakIntPoint (Variables|/Game/PathTracer/Showcase/ShowcaseBlueprints/BP_Grid.BP_Grid_C|GetGridSize _gridactor))) (LocalVariables|GetCellNumLOCAL)) :Option%201 (+ (+ (LocalVariables|GetCellNumLOCAL) (- (.X (Utilities|Struct|BreakIntPoint (Default|GetGridCoordinatesbyCellNum _gridactor (LocalVariables|GetCellNumLOCAL)))) 1)) 1) :Option%202 (+ (+ (.X (Utilities|Struct|BreakIntPoint (Default|GetGridCoordinatesbyCellNum _gridactor (LocalVariables|GetCellNumLOCAL)))) (.Y (Utilities|Struct|BreakIntPoint (Variables|/Game/PathTracer/Showcase/ShowcaseBlueprints/BP_Grid.BP_Grid_C|GetGridSize _gridactor))) (LocalVariables|GetCellNumLOCAL)) 1) :Option%203 (+ (+ (.X (Utilities|Struct|BreakIntPoint (Default|GetGridCoordinatesbyCellNum _gridactor (LocalVariables|GetCellNumLOCAL)))) (.Y (Utilities|Struct|BreakIntPoint (Variables|/Game/PathTracer/Showcase/ShowcaseBlueprints/BP_Grid.BP_Grid_C|GetGridSize _gridactor))) (LocalVariables|GetCellNumLOCAL)) 1)) (Utilities|Select :Index (LocalVariables|GetDirectionLOCAL) :Option%200 (+ (LocalVariables|GetCellNumLOCAL) (- (.X (Utilities|Struct|BreakIntPoint (Default|GetGridCoordinatesbyCellNum _gridactor (LocalVariables|GetCellNumLOCAL)))) 1)) :Option%201 (+ (LocalVariables|GetCellNumLOCAL) (- (.X (Utilities|Struct|BreakIntPoint (Default|GetGridCoordinatesbyCellNum _gridactor (LocalVariables|GetCellNumLOCAL)))) 1)) :Option%202 (+ (+ (LocalVariables|GetCellNumLOCAL) (- (.X (Utilities|Struct|BreakIntPoint (Default|GetGridCoordinatesbyCellNum _gridactor (LocalVariables|GetCellNumLOCAL)))) 1)) 1) :Option%203 (+ (.X (Utilities|Struct|BreakIntPoint (Default|GetGridCoordinatesbyCellNum _gridactor (LocalVariables|GetCellNumLOCAL)))) (.Y (Utilities|Struct|BreakIntPoint (Variables|/Game/PathTracer/Showcase/ShowcaseBlueprints/BP_Grid.BP_Grid_C|GetGridSize _gridactor))) (LocalVariables|GetCellNumLOCAL))))))))
  (Utilities|Array|Add (Variables|Default|GetConnectedWith) (Utilities|Struct|MakeS_RibData (.Y (Utilities|Struct|BreakIntPoint (Utilities|Select :Index (LocalVariables|GetDirectionLOCAL) :Option%200 (Utilities|Struct|MakeIntPoint (Utilities|Select :Index (LocalVariables|GetDirectionLOCAL) :Option%200 (+ (.X (Utilities|Struct|BreakIntPoint (Default|GetGridCoordinatesbyCellNum _gridactor (LocalVariables|GetCellNumLOCAL)))) (.Y (Utilities|Struct|BreakIntPoint (Variables|/Game/PathTracer/Showcase/ShowcaseBlueprints/BP_Grid.BP_Grid_C|GetGridSize _gridactor))) (LocalVariables|GetCellNumLOCAL)) :Option%201 (+ (+ (LocalVariables|GetCellNumLOCAL) (- (.X (Utilities|Struct|BreakIntPoint (Default|GetGridCoordinatesbyCellNum _gridactor (LocalVariables|GetCellNumLOCAL)))) 1)) 1) :Option%202 (+ (+ (.X (Utilities|Struct|BreakIntPoint (Default|GetGridCoordinatesbyCellNum _gridactor (LocalVariables|GetCellNumLOCAL)))) (.Y (Utilities|Struct|BreakIntPoint (Variables|/Game/PathTracer/Showcase/ShowcaseBlueprints/BP_Grid.BP_Grid_C|GetGridSize _gridactor))) (LocalVariables|GetCellNumLOCAL)) 1) :Option%203 (+ (+ (.X (Utilities|Struct|BreakIntPoint (Default|GetGridCoordinatesbyCellNum _gridactor (LocalVariables|GetCellNumLOCAL)))) (.Y (Utilities|Struct|BreakIntPoint (Variables|/Game/PathTracer/Showcase/ShowcaseBlueprints/BP_Grid.BP_Grid_C|GetGridSize _gridactor))) (LocalVariables|GetCellNumLOCAL)) 1)) (Utilities|Select :Index (LocalVariables|GetDirectionLOCAL) :Option%200 (+ (LocalVariables|GetCellNumLOCAL) (- (.X (Utilities|Struct|BreakIntPoint (Default|GetGridCoordinatesbyCellNum _gridactor (LocalVariables|GetCellNumLOCAL)))) 1)) :Option%201 (+ (LocalVariables|GetCellNumLOCAL) (- (.X (Utilities|Struct|BreakIntPoint (Default|GetGridCoordinatesbyCellNum _gridactor (LocalVariables|GetCellNumLOCAL)))) 1)) :Option%202 (+ (+ (LocalVariables|GetCellNumLOCAL) (- (.X (Utilities|Struct|BreakIntPoint (Default|GetGridCoordinatesbyCellNum _gridactor (LocalVariables|GetCellNumLOCAL)))) 1)) 1) :Option%203 (+ (.X (Utilities|Struct|BreakIntPoint (Default|GetGridCoordinatesbyCellNum _gridactor (LocalVariables|GetCellNumLOCAL)))) (.Y (Utilities|Struct|BreakIntPoint (Variables|/Game/PathTracer/Showcase/ShowcaseBlueprints/BP_Grid.BP_Grid_C|GetGridSize _gridactor))) (LocalVariables|GetCellNumLOCAL)))) :Option%201 (Utilities|Struct|MakeIntPoint (Utilities|Select :Index (LocalVariables|GetDirectionLOCAL) :Option%200 (+ (LocalVariables|GetCellNumLOCAL) (- (.X (Utilities|Struct|BreakIntPoint (Default|GetGridCoordinatesbyCellNum _gridactor (LocalVariables|GetCellNumLOCAL)))) 1)) :Option%201 (+ (LocalVariables|GetCellNumLOCAL) (- (.X (Utilities|Struct|BreakIntPoint (Default|GetGridCoordinatesbyCellNum _gridactor (LocalVariables|GetCellNumLOCAL)))) 1)) :Option%202 (+ (+ (LocalVariables|GetCellNumLOCAL) (- (.X (Utilities|Struct|BreakIntPoint (Default|GetGridCoordinatesbyCellNum _gridactor (LocalVariables|GetCellNumLOCAL)))) 1)) 1) :Option%203 (+ (.X (Utilities|Struct|BreakIntPoint (Default|GetGridCoordinatesbyCellNum _gridactor (LocalVariables|GetCellNumLOCAL)))) (.Y (Utilities|Struct|BreakIntPoint (Variables|/Game/PathTracer/Showcase/ShowcaseBlueprints/BP_Grid.BP_Grid_C|GetGridSize _gridactor))) (LocalVariables|GetCellNumLOCAL))) (Utilities|Select :Index (LocalVariables|GetDirectionLOCAL) :Option%200 (+ (.X (Utilities|Struct|BreakIntPoint (Default|GetGridCoordinatesbyCellNum _gridactor (LocalVariables|GetCellNumLOCAL)))) (.Y (Utilities|Struct|BreakIntPoint (Variables|/Game/PathTracer/Showcase/ShowcaseBlueprints/BP_Grid.BP_Grid_C|GetGridSize _gridactor))) (LocalVariables|GetCellNumLOCAL)) :Option%201 (+ (+ (LocalVariables|GetCellNumLOCAL) (- (.X (Utilities|Struct|BreakIntPoint (Default|GetGridCoordinatesbyCellNum _gridactor (LocalVariables|GetCellNumLOCAL)))) 1)) 1) :Option%202 (+ (+ (.X (Utilities|Struct|BreakIntPoint (Default|GetGridCoordinatesbyCellNum _gridactor (LocalVariables|GetCellNumLOCAL)))) (.Y (Utilities|Struct|BreakIntPoint (Variables|/Game/PathTracer/Showcase/ShowcaseBlueprints/BP_Grid.BP_Grid_C|GetGridSize _gridactor))) (LocalVariables|GetCellNumLOCAL)) 1) :Option%203 (+ (+ (.X (Utilities|Struct|BreakIntPoint (Default|GetGridCoordinatesbyCellNum _gridactor (LocalVariables|GetCellNumLOCAL)))) (.Y (Utilities|Struct|BreakIntPoint (Variables|/Game/PathTracer/Showcase/ShowcaseBlueprints/BP_Grid.BP_Grid_C|GetGridSize _gridactor))) (LocalVariables|GetCellNumLOCAL)) 1))) :Option%202 (Utilities|Struct|MakeIntPoint (Utilities|Select :Index (LocalVariables|GetDirectionLOCAL) :Option%200 (+ (LocalVariables|GetCellNumLOCAL) (- (.X (Utilities|Struct|BreakIntPoint (Default|GetGridCoordinatesbyCellNum _gridactor (LocalVariables|GetCellNumLOCAL)))) 1)) :Option%201 (+ (LocalVariables|GetCellNumLOCAL) (- (.X (Utilities|Struct|BreakIntPoint (Default|GetGridCoordinatesbyCellNum _gridactor (LocalVariables|GetCellNumLOCAL)))) 1)) :Option%202 (+ (+ (LocalVariables|GetCellNumLOCAL) (- (.X (Utilities|Struct|BreakIntPoint (Default|GetGridCoordinatesbyCellNum _gridactor (LocalVariables|GetCellNumLOCAL)))) 1)) 1) :Option%203 (+ (.X (Utilities|Struct|BreakIntPoint (Default|GetGridCoordinatesbyCellNum _gridactor (LocalVariables|GetCellNumLOCAL)))) (.Y (Utilities|Struct|BreakIntPoint (Variables|/Game/PathTracer/Showcase/ShowcaseBlueprints/BP_Grid.BP_Grid_C|GetGridSize _gridactor))) (LocalVariables|GetCellNumLOCAL))) (Utilities|Select :Index (LocalVariables|GetDirectionLOCAL) :Option%200 (+ (.X (Utilities|Struct|BreakIntPoint (Default|GetGridCoordinatesbyCellNum _gridactor (LocalVariables|GetCellNumLOCAL)))) (.Y (Utilities|Struct|BreakIntPoint (Variables|/Game/PathTracer/Showcase/ShowcaseBlueprints/BP_Grid.BP_Grid_C|GetGridSize _gridactor))) (LocalVariables|GetCellNumLOCAL)) :Option%201 (+ (+ (LocalVariables|GetCellNumLOCAL) (- (.X (Utilities|Struct|BreakIntPoint (Default|GetGridCoordinatesbyCellNum _gridactor (LocalVariables|GetCellNumLOCAL)))) 1)) 1) :Option%202 (+ (+ (.X (Utilities|Struct|BreakIntPoint (Default|GetGridCoordinatesbyCellNum _gridactor (LocalVariables|GetCellNumLOCAL)))) (.Y (Utilities|Struct|BreakIntPoint (Variables|/Game/PathTracer/Showcase/ShowcaseBlueprints/BP_Grid.BP_Grid_C|GetGridSize _gridactor))) (LocalVariables|GetCellNumLOCAL)) 1) :Option%203 (+ (+ (.X (Utilities|Struct|BreakIntPoint (Default|GetGridCoordinatesbyCellNum _gridactor (LocalVariables|GetCellNumLOCAL)))) (.Y (Utilities|Struct|BreakIntPoint (Variables|/Game/PathTracer/Showcase/ShowcaseBlueprints/BP_Grid.BP_Grid_C|GetGridSize _gridactor))) (LocalVariables|GetCellNumLOCAL)) 1))) :Option%203 (Utilities|Struct|MakeIntPoint (Utilities|Select :Index (LocalVariables|GetDirectionLOCAL) :Option%200 (+ (.X (Utilities|Struct|BreakIntPoint (Default|GetGridCoordinatesbyCellNum _gridactor (LocalVariables|GetCellNumLOCAL)))) (.Y (Utilities|Struct|BreakIntPoint (Variables|/Game/PathTracer/Showcase/ShowcaseBlueprints/BP_Grid.BP_Grid_C|GetGridSize _gridactor))) (LocalVariables|GetCellNumLOCAL)) :Option%201 (+ (+ (LocalVariables|GetCellNumLOCAL) (- (.X (Utilities|Struct|BreakIntPoint (Default|GetGridCoordinatesbyCellNum _gridactor (LocalVariables|GetCellNumLOCAL)))) 1)) 1) :Option%202 (+ (+ (.X (Utilities|Struct|BreakIntPoint (Default|GetGridCoordinatesbyCellNum _gridactor (LocalVariables|GetCellNumLOCAL)))) (.Y (Utilities|Struct|BreakIntPoint (Variables|/Game/PathTracer/Showcase/ShowcaseBlueprints/BP_Grid.BP_Grid_C|GetGridSize _gridactor))) (LocalVariables|GetCellNumLOCAL)) 1) :Option%203 (+ (+ (.X (Utilities|Struct|BreakIntPoint (Default|GetGridCoordinatesbyCellNum _gridactor (LocalVariables|GetCellNumLOCAL)))) (.Y (Utilities|Struct|BreakIntPoint (Variables|/Game/PathTracer/Showcase/ShowcaseBlueprints/BP_Grid.BP_Grid_C|GetGridSize _gridactor))) (LocalVariables|GetCellNumLOCAL)) 1)) (Utilities|Select :Index (LocalVariables|GetDirectionLOCAL) :Option%200 (+ (LocalVariables|GetCellNumLOCAL) (- (.X (Utilities|Struct|BreakIntPoint (Default|GetGridCoordinatesbyCellNum _gridactor (LocalVariables|GetCellNumLOCAL)))) 1)) :Option%201 (+ (LocalVariables|GetCellNumLOCAL) (- (.X (Utilities|Struct|BreakIntPoint (Default|GetGridCoordinatesbyCellNum _gridactor (LocalVariables|GetCellNumLOCAL)))) 1)) :Option%202 (+ (+ (LocalVariables|GetCellNumLOCAL) (- (.X (Utilities|Struct|BreakIntPoint (Default|GetGridCoordinatesbyCellNum _gridactor (LocalVariables|GetCellNumLOCAL)))) 1)) 1) :Option%203 (+ (.X (Utilities|Struct|BreakIntPoint (Default|GetGridCoordinatesbyCellNum _gridactor (LocalVariables|GetCellNumLOCAL)))) (.Y (Utilities|Struct|BreakIntPoint (Variables|/Game/PathTracer/Showcase/ShowcaseBlueprints/BP_Grid.BP_Grid_C|GetGridSize _gridactor))) (LocalVariables|GetCellNumLOCAL))))))) (LocalVariables|GetDirectionLOCAL)))
  ;;[0.09538 0.5938 0 0.15 16] If the point is already in the array, add point to array DuplicatePoints
  ;;
  ;; Further, knowing that the point is duplicated, it will be possible to choose the direction of bypassing the perimeter
  (if (LocalVariables|GetPointAlreadyInArrayLOCAL)
    (Utilities|Array|Add (Variables|Default|GetDuplicatePoints) (.X (Utilities|Struct|BreakIntPoint (Utilities|Select :Index (LocalVariables|GetDirectionLOCAL) :Option%200 (Utilities|Struct|MakeIntPoint (Utilities|Select :Index (LocalVariables|GetDirectionLOCAL) :Option%200 (+ (.X (Utilities|Struct|BreakIntPoint (Default|GetGridCoordinatesbyCellNum _gridactor (LocalVariables|GetCellNumLOCAL)))) (.Y (Utilities|Struct|BreakIntPoint (Variables|/Game/PathTracer/Showcase/ShowcaseBlueprints/BP_Grid.BP_Grid_C|GetGridSize _gridactor))) (LocalVariables|GetCellNumLOCAL)) :Option%201 (+ (+ (LocalVariables|GetCellNumLOCAL) (- (.X (Utilities|Struct|BreakIntPoint (Default|GetGridCoordinatesbyCellNum _gridactor (LocalVariables|GetCellNumLOCAL)))) 1)) 1) :Option%202 (+ (+ (.X (Utilities|Struct|BreakIntPoint (Default|GetGridCoordinatesbyCellNum _gridactor (LocalVariables|GetCellNumLOCAL)))) (.Y (Utilities|Struct|BreakIntPoint (Variables|/Game/PathTracer/Showcase/ShowcaseBlueprints/BP_Grid.BP_Grid_C|GetGridSize _gridactor))) (LocalVariables|GetCellNumLOCAL)) 1) :Option%203 (+ (+ (.X (Utilities|Struct|BreakIntPoint (Default|GetGridCoordinatesbyCellNum _gridactor (LocalVariables|GetCellNumLOCAL)))) (.Y (Utilities|Struct|BreakIntPoint (Variables|/Game/PathTracer/Showcase/ShowcaseBlueprints/BP_Grid.BP_Grid_C|GetGridSize _gridactor))) (LocalVariables|GetCellNumLOCAL)) 1)) (Utilities|Select :Index (LocalVariables|GetDirectionLOCAL) :Option%200 (+ (LocalVariables|GetCellNumLOCAL) (- (.X (Utilities|Struct|BreakIntPoint (Default|GetGridCoordinatesbyCellNum _gridactor (LocalVariables|GetCellNumLOCAL)))) 1)) :Option%201 (+ (LocalVariables|GetCellNumLOCAL) (- (.X (Utilities|Struct|BreakIntPoint (Default|GetGridCoordinatesbyCellNum _gridactor (LocalVariables|GetCellNumLOCAL)))) 1)) :Option%202 (+ (+ (LocalVariables|GetCellNumLOCAL) (- (.X (Utilities|Struct|BreakIntPoint (Default|GetGridCoordinatesbyCellNum _gridactor (LocalVariables|GetCellNumLOCAL)))) 1)) 1) :Option%203 (+ (.X (Utilities|Struct|BreakIntPoint (Default|GetGridCoordinatesbyCellNum _gridactor (LocalVariables|GetCellNumLOCAL)))) (.Y (Utilities|Struct|BreakIntPoint (Variables|/Game/PathTracer/Showcase/ShowcaseBlueprints/BP_Grid.BP_Grid_C|GetGridSize _gridactor))) (LocalVariables|GetCellNumLOCAL)))) :Option%201 (Utilities|Struct|MakeIntPoint (Utilities|Select :Index (LocalVariables|GetDirectionLOCAL) :Option%200 (+ (LocalVariables|GetCellNumLOCAL) (- (.X (Utilities|Struct|BreakIntPoint (Default|GetGridCoordinatesbyCellNum _gridactor (LocalVariables|GetCellNumLOCAL)))) 1)) :Option%201 (+ (LocalVariables|GetCellNumLOCAL) (- (.X (Utilities|Struct|BreakIntPoint (Default|GetGridCoordinatesbyCellNum _gridactor (LocalVariables|GetCellNumLOCAL)))) 1)) :Option%202 (+ (+ (LocalVariables|GetCellNumLOCAL) (- (.X (Utilities|Struct|BreakIntPoint (Default|GetGridCoordinatesbyCellNum _gridactor (LocalVariables|GetCellNumLOCAL)))) 1)) 1) :Option%203 (+ (.X (Utilities|Struct|BreakIntPoint (Default|GetGridCoordinatesbyCellNum _gridactor (LocalVariables|GetCellNumLOCAL)))) (.Y (Utilities|Struct|BreakIntPoint (Variables|/Game/PathTracer/Showcase/ShowcaseBlueprints/BP_Grid.BP_Grid_C|GetGridSize _gridactor))) (LocalVariables|GetCellNumLOCAL))) (Utilities|Select :Index (LocalVariables|GetDirectionLOCAL) :Option%200 (+ (.X (Utilities|Struct|BreakIntPoint (Default|GetGridCoordinatesbyCellNum _gridactor (LocalVariables|GetCellNumLOCAL)))) (.Y (Utilities|Struct|BreakIntPoint (Variables|/Game/PathTracer/Showcase/ShowcaseBlueprints/BP_Grid.BP_Grid_C|GetGridSize _gridactor))) (LocalVariables|GetCellNumLOCAL)) :Option%201 (+ (+ (LocalVariables|GetCellNumLOCAL) (- (.X (Utilities|Struct|BreakIntPoint (Default|GetGridCoordinatesbyCellNum _gridactor (LocalVariables|GetCellNumLOCAL)))) 1)) 1) :Option%202 (+ (+ (.X (Utilities|Struct|BreakIntPoint (Default|GetGridCoordinatesbyCellNum _gridactor (LocalVariables|GetCellNumLOCAL)))) (.Y (Utilities|Struct|BreakIntPoint (Variables|/Game/PathTracer/Showcase/ShowcaseBlueprints/BP_Grid.BP_Grid_C|GetGridSize _gridactor))) (LocalVariables|GetCellNumLOCAL)) 1) :Option%203 (+ (+ (.X (Utilities|Struct|BreakIntPoint (Default|GetGridCoordinatesbyCellNum _gridactor (LocalVariables|GetCellNumLOCAL)))) (.Y (Utilities|Struct|BreakIntPoint (Variables|/Game/PathTracer/Showcase/ShowcaseBlueprints/BP_Grid.BP_Grid_C|GetGridSize _gridactor))) (LocalVariables|GetCellNumLOCAL)) 1))) :Option%202 (Utilities|Struct|MakeIntPoint (Utilities|Select :Index (LocalVariables|GetDirectionLOCAL) :Option%200 (+ (LocalVariables|GetCellNumLOCAL) (- (.X (Utilities|Struct|BreakIntPoint (Default|GetGridCoordinatesbyCellNum _gridactor (LocalVariables|GetCellNumLOCAL)))) 1)) :Option%201 (+ (LocalVariables|GetCellNumLOCAL) (- (.X (Utilities|Struct|BreakIntPoint (Default|GetGridCoordinatesbyCellNum _gridactor (LocalVariables|GetCellNumLOCAL)))) 1)) :Option%202 (+ (+ (LocalVariables|GetCellNumLOCAL) (- (.X (Utilities|Struct|BreakIntPoint (Default|GetGridCoordinatesbyCellNum _gridactor (LocalVariables|GetCellNumLOCAL)))) 1)) 1) :Option%203 (+ (.X (Utilities|Struct|BreakIntPoint (Default|GetGridCoordinatesbyCellNum _gridactor (LocalVariables|GetCellNumLOCAL)))) (.Y (Utilities|Struct|BreakIntPoint (Variables|/Game/PathTracer/Showcase/ShowcaseBlueprints/BP_Grid.BP_Grid_C|GetGridSize _gridactor))) (LocalVariables|GetCellNumLOCAL))) (Utilities|Select :Index (LocalVariables|GetDirectionLOCAL) :Option%200 (+ (.X (Utilities|Struct|BreakIntPoint (Default|GetGridCoordinatesbyCellNum _gridactor (LocalVariables|GetCellNumLOCAL)))) (.Y (Utilities|Struct|BreakIntPoint (Variables|/Game/PathTracer/Showcase/ShowcaseBlueprints/BP_Grid.BP_Grid_C|GetGridSize _gridactor))) (LocalVariables|GetCellNumLOCAL)) :Option%201 (+ (+ (LocalVariables|GetCellNumLOCAL) (- (.X (Utilities|Struct|BreakIntPoint (Default|GetGridCoordinatesbyCellNum _gridactor (LocalVariables|GetCellNumLOCAL)))) 1)) 1) :Option%202 (+ (+ (.X (Utilities|Struct|BreakIntPoint (Default|GetGridCoordinatesbyCellNum _gridactor (LocalVariables|GetCellNumLOCAL)))) (.Y (Utilities|Struct|BreakIntPoint (Variables|/Game/PathTracer/Showcase/ShowcaseBlueprints/BP_Grid.BP_Grid_C|GetGridSize _gridactor))) (LocalVariables|GetCellNumLOCAL)) 1) :Option%203 (+ (+ (.X (Utilities|Struct|BreakIntPoint (Default|GetGridCoordinatesbyCellNum _gridactor (LocalVariables|GetCellNumLOCAL)))) (.Y (Utilities|Struct|BreakIntPoint (Variables|/Game/PathTracer/Showcase/ShowcaseBlueprints/BP_Grid.BP_Grid_C|GetGridSize _gridactor))) (LocalVariables|GetCellNumLOCAL)) 1))) :Option%203 (Utilities|Struct|MakeIntPoint (Utilities|Select :Index (LocalVariables|GetDirectionLOCAL) :Option%200 (+ (.X (Utilities|Struct|BreakIntPoint (Default|GetGridCoordinatesbyCellNum _gridactor (LocalVariables|GetCellNumLOCAL)))) (.Y (Utilities|Struct|BreakIntPoint (Variables|/Game/PathTracer/Showcase/ShowcaseBlueprints/BP_Grid.BP_Grid_C|GetGridSize _gridactor))) (LocalVariables|GetCellNumLOCAL)) :Option%201 (+ (+ (LocalVariables|GetCellNumLOCAL) (- (.X (Utilities|Struct|BreakIntPoint (Default|GetGridCoordinatesbyCellNum _gridactor (LocalVariables|GetCellNumLOCAL)))) 1)) 1) :Option%202 (+ (+ (.X (Utilities|Struct|BreakIntPoint (Default|GetGridCoordinatesbyCellNum _gridactor (LocalVariables|GetCellNumLOCAL)))) (.Y (Utilities|Struct|BreakIntPoint (Variables|/Game/PathTracer/Showcase/ShowcaseBlueprints/BP_Grid.BP_Grid_C|GetGridSize _gridactor))) (LocalVariables|GetCellNumLOCAL)) 1) :Option%203 (+ (+ (.X (Utilities|Struct|BreakIntPoint (Default|GetGridCoordinatesbyCellNum _gridactor (LocalVariables|GetCellNumLOCAL)))) (.Y (Utilities|Struct|BreakIntPoint (Variables|/Game/PathTracer/Showcase/ShowcaseBlueprints/BP_Grid.BP_Grid_C|GetGridSize _gridactor))) (LocalVariables|GetCellNumLOCAL)) 1)) (Utilities|Select :Index (LocalVariables|GetDirectionLOCAL) :Option%200 (+ (LocalVariables|GetCellNumLOCAL) (- (.X (Utilities|Struct|BreakIntPoint (Default|GetGridCoordinatesbyCellNum _gridactor (LocalVariables|GetCellNumLOCAL)))) 1)) :Option%201 (+ (LocalVariables|GetCellNumLOCAL) (- (.X (Utilities|Struct|BreakIntPoint (Default|GetGridCoordinatesbyCellNum _gridactor (LocalVariables|GetCellNumLOCAL)))) 1)) :Option%202 (+ (+ (LocalVariables|GetCellNumLOCAL) (- (.X (Utilities|Struct|BreakIntPoint (Default|GetGridCoordinatesbyCellNum _gridactor (LocalVariables|GetCellNumLOCAL)))) 1)) 1) :Option%203 (+ (.X (Utilities|Struct|BreakIntPoint (Default|GetGridCoordinatesbyCellNum _gridactor (LocalVariables|GetCellNumLOCAL)))) (.Y (Utilities|Struct|BreakIntPoint (Variables|/Game/PathTracer/Showcase/ShowcaseBlueprints/BP_Grid.BP_Grid_C|GetGridSize _gridactor))) (LocalVariables|GetCellNumLOCAL))))))))))

(fn GetPathTracer
  (bind _pathtrecersarray (Variables|Default|GetPathTrecersArray))
  (bind _pathusingamount (Variables|Default|GetPathUsingAmount))
  (bind _returnvalue (- _pathusingamount 1))
  (bind _output (Utilities|Array|Get(acopy) _pathtrecersarray _returnvalue))
  (if (> (Utilities|Array|Length (Variables|Default|GetPathTrecersArray)) (Variables|Default|GetPathUsingAmount))
    (Math|Integer|IncrementInt (Variables|Default|GetPathUsingAmount)
      (:%20%20
        (if true
          (Rendering|SetActorHiddenInGame _output false)
          (return _output))))
    (else
      (bind _returnvalue_2 (AddComponent|AddChildActorComponent false))
      (ChildActorComponent|SetChildActorClass _returnvalue_2 (Variables|Default|GetPathTracerClass))
      (bind _asbp_path_tracer (Utilities|Casting|CastToBP_PathTracer (Variables|/Script/Engine.ChildActorComponent|GetChildActor _returnvalue_2)))
      (Utilities|Array|Add (Variables|Default|GetPathTrecersArray) _asbp_path_tracer)
      (Math|Integer|IncrementInt (Variables|Default|GetPathUsingAmount)
        (:%20%20
          (return _asbp_path_tracer))))))

(fn ResetPathTrecers
  (for _array_element (Variables|Default|GetPathTrecersArray)
    (Rendering|SetActorHiddenInGame _array_element true))
  (Variables|Default|SetPathUsingAmount 0))