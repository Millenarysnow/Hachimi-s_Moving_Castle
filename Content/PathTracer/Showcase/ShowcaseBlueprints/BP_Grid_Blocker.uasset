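; BP_Grid_Blocker is a resizable box blocker whose construction script turns editor scaling into stepped size changes.
; Scaling an axis up or down moves BlockerSize by ScaleStep, clamped at zero, then actor scale resets to one.
; BlockerSize drives the box extent, static mesh scale and billboard height above the box.
; A bounding-radius calculation exists but is unconnected, and no runtime logic is present.
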(fn ConstructionScript
  (bind _returnvalue (Class|Actor|GetActorRelativeScale3D))
  (bind (_x _y _z) (Math|Vector|BreakVector _returnvalue))
  (bind (_x_2 _y_2 _z_2) (Math|Vector|BreakVector _returnvalue))
  (if (Math|Vector|Equal(Vector) (Class|Actor|GetActorRelativeScale3D) "1.000000,1.000000,1.000000" 0.01)
    _
    (else
      (Variables|Default|SetBlockerSize (Math|Vector|MakeVector (Math|Float|SelectFloat (Math|Float|SelectFloat (.X (Math|Vector|BreakVector (Variables|Default|GetBlockerSize))) (+ (.X (Math|Vector|BreakVector (Variables|Default|GetBlockerSize))) (* (Math|Float|SelectFloat -1.0 1.0 (< _x 1.0)) (Variables|Default|GetScaleStep))) (== _x_2 1.0)) 0.0 (>= (Math|Float|SelectFloat (.X (Math|Vector|BreakVector (Variables|Default|GetBlockerSize))) (+ (.X (Math|Vector|BreakVector (Variables|Default|GetBlockerSize))) (* (Math|Float|SelectFloat -1.0 1.0 (< _x 1.0)) (Variables|Default|GetScaleStep))) (== _x_2 1.0)) 0.0)) (Math|Float|SelectFloat (Math|Float|SelectFloat (.Y (Math|Vector|BreakVector (Variables|Default|GetBlockerSize))) (+ (.Y (Math|Vector|BreakVector (Variables|Default|GetBlockerSize))) (* (Math|Float|SelectFloat -1.0 1.0 (< _y 1.0)) (Variables|Default|GetScaleStep))) (== _y_2 1.0)) 0.0 (>= (Math|Float|SelectFloat (.Y (Math|Vector|BreakVector (Variables|Default|GetBlockerSize))) (+ (.Y (Math|Vector|BreakVector (Variables|Default|GetBlockerSize))) (* (Math|Float|SelectFloat -1.0 1.0 (< _y 1.0)) (Variables|Default|GetScaleStep))) (== _y_2 1.0)) 0.0)) (Math|Float|SelectFloat (Math|Float|SelectFloat (.Z (Math|Vector|BreakVector (Variables|Default|GetBlockerSize))) (+ (.Z (Math|Vector|BreakVector (Variables|Default|GetBlockerSize))) (* (Math|Float|SelectFloat -1.0 1.0 (< _z 1.0)) (Variables|Default|GetScaleStep))) (== _z_2 1.0)) 0.0 (>= (Math|Float|SelectFloat (.Z (Math|Vector|BreakVector (Variables|Default|GetBlockerSize))) (+ (.Z (Math|Vector|BreakVector (Variables|Default|GetBlockerSize))) (* (Math|Float|SelectFloat -1.0 1.0 (< _z 1.0)) (Variables|Default|GetScaleStep))) (== _z_2 1.0)) 0.0))))))
  (Components|Box|SetBoxExtent (Variables|Default|GetBox) (* (Variables|Default|GetBlockerSize) 0.5) true)
  (Transformation|SetActorScale3D "1.000000,1.000000,1.000000")
  (Transformation|SetRelativeScale3D (Variables|Default|GetStaticMesh) (/ (Math|Vector|MakeVector (Math|Float|SelectFloat (Math|Float|SelectFloat (.X (Math|Vector|BreakVector (Variables|Default|GetBlockerSize))) (+ (.X (Math|Vector|BreakVector (Variables|Default|GetBlockerSize))) (* (Math|Float|SelectFloat -1.0 1.0 (< _x 1.0)) (Variables|Default|GetScaleStep))) (== _x_2 1.0)) 0.0 (>= (Math|Float|SelectFloat (.X (Math|Vector|BreakVector (Variables|Default|GetBlockerSize))) (+ (.X (Math|Vector|BreakVector (Variables|Default|GetBlockerSize))) (* (Math|Float|SelectFloat -1.0 1.0 (< _x 1.0)) (Variables|Default|GetScaleStep))) (== _x_2 1.0)) 0.0)) (Math|Float|SelectFloat (Math|Float|SelectFloat (.Y (Math|Vector|BreakVector (Variables|Default|GetBlockerSize))) (+ (.Y (Math|Vector|BreakVector (Variables|Default|GetBlockerSize))) (* (Math|Float|SelectFloat -1.0 1.0 (< _y 1.0)) (Variables|Default|GetScaleStep))) (== _y_2 1.0)) 0.0 (>= (Math|Float|SelectFloat (.Y (Math|Vector|BreakVector (Variables|Default|GetBlockerSize))) (+ (.Y (Math|Vector|BreakVector (Variables|Default|GetBlockerSize))) (* (Math|Float|SelectFloat -1.0 1.0 (< _y 1.0)) (Variables|Default|GetScaleStep))) (== _y_2 1.0)) 0.0)) (Math|Float|SelectFloat (Math|Float|SelectFloat (.Z (Math|Vector|BreakVector (Variables|Default|GetBlockerSize))) (+ (.Z (Math|Vector|BreakVector (Variables|Default|GetBlockerSize))) (* (Math|Float|SelectFloat -1.0 1.0 (< _z 1.0)) (Variables|Default|GetScaleStep))) (== _z_2 1.0)) 0.0 (>= (Math|Float|SelectFloat (.Z (Math|Vector|BreakVector (Variables|Default|GetBlockerSize))) (+ (.Z (Math|Vector|BreakVector (Variables|Default|GetBlockerSize))) (* (Math|Float|SelectFloat -1.0 1.0 (< _z 1.0)) (Variables|Default|GetScaleStep))) (== _z_2 1.0)) 0.0))) 1e+02))
  (Transformation|SetRelativeLocation (Variables|Default|GetBillboard) (Math|Vector|MakeVector 0.0 0.0 (+ (* (.Z (Math|Vector|BreakVector (Variables|Default|GetBlockerSize))) 0.5) 5e+01)) false false))